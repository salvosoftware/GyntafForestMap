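; Editor-placed spline measuring tool that shows the spline's length as meter and foot text labels.
; The construction script optionally tiles spline meshes in fixed-length sections, with tangents clamped to section length, optional X-scale-driven sizing and a full-length-only mode.
; It multiplies spline length by a scale factor, converts it to several metric and imperial units, then colors, fills and toggles the labels.
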(fn `GetEndPosTangent`
  (params (index :type Integer))
  (returns (Position :type "Vector Structure") (Tangent :type "Vector Structure"))
  (bind _returnvalue (* (+ index 1) (`self.SectionLength`)))
  (return (`SplineComponent.GetLocationAtDistanceAlongSpline` (`self.Spline`) _returnvalue "Local") (`KismetMathLibrary.ClampVectorSize` (`SplineComponent.GetTangentAtDistanceAlongSpline` (`self.Spline`) _returnvalue "Local") 0.0 (`self.SectionLength`))))

(fn `GetStartPosTangent`
  (params (index :type Integer))
  (returns (position :type "Vector Structure") (Tangent :type "Vector Structure"))
  (bind _sectionlength (`self.SectionLength`))
  (bind _returnvalue (* index _sectionlength))
  (return (`SplineComponent.GetLocationAtDistanceAlongSpline` (`self.Spline`) _returnvalue "Local") (`KismetMathLibrary.ClampVectorSize` (`SplineComponent.GetTangentAtDistanceAlongSpline` (`self.Spline`) _returnvalue "Local") 0.0 _sectionlength)))

(fn `UserConstructionScript`
  (bind _returnvalue_x (`KismetMathLibrary.BreakVector` (`self.GetActorScale3D`)))
  (`|ExecutionSequence`
    (:`then_0`
      (if (`self.Use Meshes?`)
        (if (`self.Allow Scaling?`)
          (set `self.SectionLength` (* _returnvalue_x 100.0)))
        (if (`self.Full length meshes?`)
          (for _index (range (`KismetMathLibrary.FTrunc` (/ (`SplineComponent.GetSplineLength` (`self.Spline`)) (`self.SectionLength`))))
            (set `self.LoopIndex` _index)
            (bind _returnvalue (`AddComponent|NODE_AddSplineMeshComponent-0` :!label _label))
            (`StaticMeshComponent.SetStaticMesh` _returnvalue (`self.Spline Mesh`))
            (`SplineMeshComponent.SetForwardAxis` _returnvalue "X" true)
            (bind (_position _tangent) (`self.GetStartPosTangent` (`self.LoopIndex`)))
            (bind (_position_2 _tangent_2) (`self.GetEndPosTangent` (`self.LoopIndex`)))
            (`SplineMeshComponent.SetStartAndEnd` _returnvalue _position _tangent _position_2 _tangent_2 true)
            (`PrimitiveComponent.SetCollisionEnabled` _returnvalue (`self.Collision`)))
          (else
            (for _index_2 (range (+ (`KismetMathLibrary.FTrunc` (/ (`SplineComponent.GetSplineLength` (`self.Spline`)) (`self.SectionLength`))) 1))
              (set `self.LoopIndex` _index_2)
              (goto _label))))))
    (:`then_1`
      (`TextRenderComponent.SetTextRenderColor` (`self.MeterAmount`) (`KismetMathLibrary.Conv_LinearColorToColor` (`self.Text Color`)))
      (`TextRenderComponent.SetTextRenderColor` (`self.MeterText`) (`KismetMathLibrary.Conv_LinearColorToColor` (`self.Text Color`)))
      (`TextRenderComponent.SetTextRenderColor` (`self.FeetText`) (`KismetMathLibrary.Conv_LinearColorToColor` (`self.Text Color`)))
      (`TextRenderComponent.SetTextRenderColor` (`self.FeetAmount`) (`KismetMathLibrary.Conv_LinearColorToColor` (`self.Text Color`)))
      (set `self.Distance` (* (`SplineComponent.GetSplineLength` self) (`self.Scale Multiplier`)))
      (set `self.Miles` (* (`self.Distance`) 6.213712e-06))
      (set `self.Feet` (/ (`self.Distance`) 30.48))
      (set `self.Inches` (* (`self.Feet`) 12.0))
      (set `self.Meters` (/ (`self.Distance`) 100.0))
      (set `self.Kilometers` (/ (`self.Distance`) 100000.0))
      (set `self.Centimeters` (`self.Distance`))
      (`TextRenderComponent.K2_SetText` (`self.MeterAmount`) (`KismetTextLibrary.Conv_StringToText` (`KismetStringLibrary.Conv_DoubleToString` (`self.Meters`))))
      (`TextRenderComponent.K2_SetText` (`self.FeetAmount`) (`KismetTextLibrary.Conv_StringToText` (`KismetStringLibrary.Conv_DoubleToString` (`self.Feet`))))
      (if (not (`self.DisplayFeet`))
        (`SceneComponent.ToggleVisibility` false)
        (`SceneComponent.ToggleVisibility` false))
      (if (not (`self.DisplayMeters`))
        (`SceneComponent.ToggleVisibility` false)
        (`SceneComponent.ToggleVisibility` false)))))