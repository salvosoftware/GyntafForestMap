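; BP_Marker is a configurable marker actor made of a colored plane symbol and a text label.
; Its construction script creates dynamic material instances for both, setting the label's color from TextColor and the plane's from SymbolColor.
; It also applies the Text string and a uniform world scale to the scene, plane and text components.
; The event graph has no active logic.
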(fn `UserConstructionScript`
  (bind _scale (`self.Scale`))
  (bind _returnvalue (`PrimitiveComponent.CreateDynamicMaterialInstance` (`self.TextRender`) 0 null "color"))
  (`MaterialInstanceDynamic.SetVectorParameterValue` _returnvalue "color" (`KismetMathLibrary.Conv_ColorToLinearColor` (`self.TextColor`)))
  (`TextRenderComponent.K2_SetText` (`self.TextRender`) (`self.Text`))
  (bind _returnvalue_2 (`PrimitiveComponent.CreateDynamicMaterialInstance` (`self.Plane`) 0 null "None"))
  (`MaterialInstanceDynamic.SetVectorParameterValue` _returnvalue_2 "color" (`self.SymbolColor`))
  (`SceneComponent.SetWorldScale3D` (`self.Scene`) (`KismetMathLibrary.MakeVector` _scale _scale _scale))
  (`SceneComponent.SetWorldScale3D` (`self.Plane`) (`KismetMathLibrary.MakeVector` _scale _scale _scale))
  (`SceneComponent.SetWorldScale3D` (`self.TextRender`) (`KismetMathLibrary.MakeVector` _scale _scale _scale)))