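; Simple editor measuring tool actor that shows the distance between PointA and PointB as text labels in meters and feet.
; The construction script scales the vector length between the points and stores it in several metric and imperial units.
; It also applies the text color, updates the meter and feet readouts, and toggles visibility when either display option is off.
; The event graph has no active logic.
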(fn `UserConstructionScript`
  (`TextRenderComponent.SetTextRenderColor` (`self.MeterAmount`) (`KismetMathLibrary.Conv_LinearColorToColor` (`self.Text Color`)))
  (`TextRenderComponent.SetTextRenderColor` (`self.FeetAmount`) (`KismetMathLibrary.Conv_LinearColorToColor` (`self.Text Color`)))
  (`TextRenderComponent.SetTextRenderColor` (`self.FeetText`) (`KismetMathLibrary.Conv_LinearColorToColor` (`self.Text Color`)))
  (`TextRenderComponent.SetTextRenderColor` (`self.MeterText`) (`KismetMathLibrary.Conv_LinearColorToColor` (`self.Text Color`)))
  (set `self.Distance` (* (`KismetMathLibrary.VSize` (- (`self.PointA`) (`self.PointB`))) (`self.Scale Multiplier`)))
  (set `self.Miles` (* (`self.Distance`) 6.213712e-06))
  (set `self.Feet` (/ (`self.Distance`) 30.48))
  (set `self.Inches` (* (`self.Feet`) 12.0))
  (set `self.Meters` (/ (`self.Distance`) 100.0))
  (set `self.Kilometers` (/ (`self.Distance`) 100000.0))
  (set `self.Centimeters` (`self.Distance`))
  (`TextRenderComponent.K2_SetText` (`self.MeterText`) (`KismetTextLibrary.Conv_StringToText` (`KismetStringLibrary.Conv_DoubleToString` (`self.Meters`))))
  (`TextRenderComponent.K2_SetText` (`self.FeetText`) (`KismetTextLibrary.Conv_StringToText` (`KismetStringLibrary.Conv_DoubleToString` (`self.Feet`))))
  (if (not (`self.DisplayMeters`))
    (`SceneComponent.ToggleVisibility` false)
    (`SceneComponent.ToggleVisibility` false))
  (if (not (`self.DisplayFeet`))
    (`SceneComponent.ToggleVisibility` false)
    (`SceneComponent.ToggleVisibility` false)))